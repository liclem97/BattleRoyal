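; BP_Mine is a mine actor that explodes once when a player character overlaps its sphere.
; The overlap is handled only on the server, which calls ShowExplosionEffect to spawn an explosion emitter and then sets Exploded.
; Exploded uses a RepNotify to switch the cube to an exploded material.
; The WhichComputer macro branches execution by authority and ownership into server, owning client or other client.
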(event `self.Sphere.OnComponentBeginOverlap`
  (params (OverlappedComponent :type "PrimitiveComponent Object Reference") (OtherActor :type "Actor Object Reference") (OtherComp :type "PrimitiveComponent Object Reference") (OtherBodyIndex :type Integer) (bFromSweep :type Boolean) (SweepResult :type "HitResult Structure (by ref)"))
  (`self.WhichComputer`
    (:`Server`
      (if (not (`self.Exploded`))
        (cast `/Game/Characters/BP_PlayerBase` OtherActor)
        (`self.ShowExplosionEffect`)
        (set `self.Exploded` true)))))

(event `ShowExplosionEffect`
  (`GameplayStatics.SpawnEmitterAtLocation` "/Game/StarterContent/Particles/P_Explosion.P_Explosion" (`self.K2_GetActorLocation`)))

(fn `OnRep_Exploded`
  (if (`self.Exploded`)
    (`PrimitiveComponent.SetMaterial` (`self.Cube`) 0 "/Game/Characters/M_Exploded.M_Exploded")))

(fn `UserConstructionScript`)