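; Player character Blueprint that handles physical hit reactions, death ragdoll, modular gear meshes and weapon spawning.
; Health changes simulate physics from the spine down the bone chain while a timeline drives the blend weight, and zero health ragdolls the body.
; Upper, lower, helmet and shoe meshes load asynchronously from item IDs via the ItemData table.
; The weapon spawn replaces the current weapon, attaching to the hand or back socket based on RifleEquipped.
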(event `self.HealthComp.OnHealthChanged`
  (params (HealthComp :type "BRHealthComponent Object Reference") (Health :type "Float (single-precision)") (HealthDelta :type "Float (single-precision)") (DamageType :type "DamageType Object Reference") (InstigatedBy :type "Controller Object Reference") (DamageCauser :type "Actor Object Reference"))
  ;[1 1 1] 피격 애니메이션
  (if (<= Health 0.0)
    (`PrimitiveComponent.SetSimulatePhysics` (`self.Mesh`) true)
    (`|ExecutionSequence`
      (:`then_0`
        (`SkeletalMeshComponent.SetAllBodiesBelowPhysicsBlendWeight` (`self.Mesh`) "Hips" 1.0 false true)
        (`PrimitiveComponent.SetCollisionEnabled` (`self.CapsuleComponent`) "NoCollision")
        (`CharacterMovementComponent.SetMovementMode` (`self.CharacterMovement`) "MOVE_None" 0))
      (:`then_1`
        (bind (_direction _blendweight) (`Timeline|ChangeBlendWeight` :!via `Stop` :!label _label)
          (:`Update`
            (`SkeletalMeshComponent.SetAllBodiesBelowPhysicsBlendWeight` (`self.Mesh`) "Spine" _blendweight false true))
          (:`Finished`
            (`SkeletalMeshComponent.SetAllBodiesBelowSimulatePhysics` (`self.Mesh`) "Spine" false true)))))
    (else
      (`SkeletalMeshComponent.SetAllBodiesBelowSimulatePhysics` (`self.Mesh`) "Spine" true true)
      (`SkeletalMeshComponent.SetAllBodiesBelowPhysicsBlendWeight` (`self.Mesh`) "Spine" 1.0 false true)
      (goto _label :!via `PlayFromStart`))))

(event `self.LoadUpperItem`
  (bind _upperitemclassid (`self.UpperItemClassID`))
  (if (!= _upperitemclassid 0)
    (bind _returnvalue (`|GetDataTableRow` "/Game/Item/ItemData.ItemData" (`KismetStringLibrary.Conv_StringToName` (`KismetStringLibrary.Conv_IntToString` _upperitemclassid)))
      (:`then`
        (bind _object (`|LoadAsset` (`.ItemSkeletalMesh` (break `ITemTableRow` _returnvalue)))
          (:`Completed`
            (bind _asskeletal_mesh (cast `SkeletalMesh` _object))
            (`SkinnedMeshComponent.SetSkinnedAssetAndUpdate` (`self.Upper`) _asskeletal_mesh false)))))))

(event `self.LoadLowerItem`
  (bind _loweritemclassid (`self.LowerItemClassID`))
  (if (!= 0 _loweritemclassid)
    (bind _returnvalue (`|GetDataTableRow` "/Game/Item/ItemData.ItemData" (`KismetStringLibrary.Conv_StringToName` (`KismetStringLibrary.Conv_IntToString` _loweritemclassid)))
      (:`then`
        (bind _object (`|LoadAsset` (`.ItemSkeletalMesh` (break `ITemTableRow` _returnvalue)))
          (:`Completed`
            (bind _asskeletal_mesh (cast `SkeletalMesh` _object))
            (`SkinnedMeshComponent.SetSkinnedAssetAndUpdate` (`self.Lower`) _asskeletal_mesh false)))))))

(event `self.LoadHelmetItem`
  (bind _helmetitemclassid (`self.HelmetItemClassID`))
  (if (!= 0 _helmetitemclassid)
    (bind _returnvalue (`|GetDataTableRow` "/Game/Item/ItemData.ItemData" (`KismetStringLibrary.Conv_StringToName` (`KismetStringLibrary.Conv_IntToString` _helmetitemclassid)))
      (:`then`
        (bind _object (`|LoadAsset` (`.ItemSkeletalMesh` (break `ITemTableRow` _returnvalue)))
          (:`Completed`
            (bind _asskeletal_mesh (cast `SkeletalMesh` _object))
            (`SkinnedMeshComponent.SetSkinnedAssetAndUpdate` (`self.Helmet`) _asskeletal_mesh false)))))))

(event `self.LoadShoesItem`
  (bind _shoesitemclassid (`self.ShoesItemClassID`))
  (if (!= 0 _shoesitemclassid)
    (bind _returnvalue (`|GetDataTableRow` "/Game/Item/ItemData.ItemData" (`KismetStringLibrary.Conv_StringToName` (`KismetStringLibrary.Conv_IntToString` _shoesitemclassid)))
      (:`then`
        (bind _object (`|LoadAsset` (`.ItemSkeletalMesh` (break `ITemTableRow` _returnvalue)))
          (:`Completed`
            (bind _asskeletal_mesh (cast `SkeletalMesh` _object))
            (`SkinnedMeshComponent.SetSkinnedAssetAndUpdate` (`self.Shoes`) _asskeletal_mesh false)))))))

(event `TESTFUNC_1`
  (`self.ServerSpawnActor`))

(event `ServerSpawnActor`
  (if (not (`KismetSystemLibrary.IsValidClass` (`self.BRWeapon`)))
    (bind _returnvalue (`|GetDataTableRow` "/Game/Item/ItemData.ItemData" (`KismetStringLibrary.Conv_StringToName` (`KismetStringLibrary.Conv_IntToString` (`self.WeaponItemClassID`))))
      (:`then`
        (bind _output_get (set `self.BRWeapon` (`.BP_Weapon` (break `ITemTableRow` _returnvalue)))))))
  (`/Engine/EditorBlueprintResources/StandardMacros.IsValid` (`self.MyWeapon`)
    (:`Is Valid`
      (`self.K2_DetachFromActor` "KeepWorld" "KeepWorld" "KeepWorld")
      (`self.K2_DestroyActor` (`self.MyWeapon`)))
    (:`Is Not Valid`
      _))
  (bind _returnvalue_2 (`|SpawnActorFromClass` _output_get (`self.GetTransform`) "AlwaysSpawn" "OverrideRootScale" self null))
  (bind _output_get_2 (set `self.MyWeapon` _returnvalue_2))
  (if (`self.bRifleEquipped`)
    (`self.K2_AttachToComponent` _output_get_2 (`self.Mesh`) "WeaponRight" "SnapToTarget" "SnapToTarget" "SnapToTarget" false)
    (else
      (`self.K2_AttachToComponent` _output_get_2 (`self.Mesh`) "WeaponBack" "SnapToTarget" "SnapToTarget" "SnapToTarget" false)))
  (set `self.BRWeapon` null))

(fn `UserConstructionScript`)